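; Master enemy AI character, set up from an EnemyDetails struct for mesh animation, speed, health, weapons and behaviour.
; It optionally roams while a looping timer looks for BP_Lisa players within sight distance.
; Combat loops AIMoveTo on the closest or furthest player and cycles attack montages, without a behaviour tree.
; Weapon overlaps damage players not already hit; taking damage lowers health, briefly shows the health bar and plays a reaction montage.
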(event Custom|Event%20Start%20Roaming
  (AI|AIMoveTo self (.RandomLocation (AI|Navigation|GetRandomReachablePointinRadius (Transformation|GetWorldLocation (Variables|Collision|GetCapsuleComponent)) 1e+03 0 0)) 0 5.0 false
    (:OnSuccess
      (Utilities|FlowControl|Delay 2.0)
      (if (not (Variables|Default|GetHas%20Target))
        (CallFunction|EventStartRoaming)))))

(event EventBeginPlay
  (bind _aswb_ai_health_bar (Utilities|Casting|CastToWB_AI_HealthBar (UserInterface|GetUserWidgetObject (Variables|Default|GetWidget))))
  (Variables|/Game/AI_CharOLD/UI/WB_AI_HealthBar.WB_AI_HealthBar_C|SetOwner _aswb_ai_health_bar self)
  (Variables|Default|SetWB%20AI%20Health%20Bar _aswb_ai_health_bar)
  (CallFunction|SetupAIMovement)
  (CallFunction|SetupAIStats)
  (CallFunction|SetupAIBehaviour)
  (Utilities|Time|SetTimerbyFunctionName 0 "Look For Player" 1.0 true)
  (CallFunction|AttachWeapon)
  (Collision|SetCollisionEnabled (Variables|Default|GetWeapon01) "NoCollision"))

(event Custom|Event%20Show%20health%20bar
  ;[1 1 1] UI
  (Default|EventShowHeathBar (Variables|Default|GetWB%20AI%20Health%20Bar))
  (Utilities|Time|SetTimerbyEvent (delegate Custom|Event%20Hide%20Health%20Bar) 3.0))

(event Custom|Event%20Hide%20Health%20Bar
  ;[1 1 1] UI
  (Default|EventHideHealthBar (Variables|Default|GetWB%20AI%20Health%20Bar)))

(event Custom|MC%20Play%20montage
  (params (AnimMontage :type Anim%20Montage%20Object%20Reference) (StartSectionName :type Name))
  ;[0 1 0.6697] Play montage
  (bind _returnvalue (Animation|PlayAnimMontage AnimMontage 1.0 StartSectionName))
  (Variables|Default|SetAnimation%20Delay _returnvalue))

(event Custom|Server%20play%20montage
  (params (AnimMontage :type Anim%20Montage%20Object%20Reference) (StartSectionName :type Name))
  ;[0 1 0.6697] Play montage
  (CallFunction|MCPlayMontage AnimMontage StartSectionName))

(event Custom|event%20stop%20rotating%20towards%20target
  (bind _returnvalue (Transformation|GetActorRotation))
  (Utilities|FlowControl|Sequence
    (:then_0
      (bind _rotation (Timeline|Timeline_0 Stop)
        (:Update
          (Utilities|IsValid (Variables|Default|GetClosest%20Player)
            (:Is%20Valid
              (Transformation|SetActorRotation (Math|Rotator|Lerp(Rotator) (Transformation|GetActorRotation) (Math|Rotator|MakeRotator (.roll _returnvalue) (.pitch _returnvalue) (.yaw (Math|Rotator|FindLookatRotation (Transformation|GetActorLocation) (Transformation|GetActorLocation (Variables|Default|GetClosest%20Player))))) _rotation true)))))))
    (:then_1
      (Utilities|FlowControl|DoOnce false) ; enters at Reset
    )))

(event Custom|Event%20rotate%20towards%20target
  (bind _returnvalue (Transformation|GetActorRotation))
  (Utilities|FlowControl|DoOnce false
    (:Completed
      (bind _rotation (Timeline|Timeline_0 PlayFromStart)
        (:Update
          (Utilities|IsValid (Variables|Default|GetClosest%20Player)
            (:Is%20Valid
              (Transformation|SetActorRotation (Math|Rotator|Lerp(Rotator) (Transformation|GetActorRotation) (Math|Rotator|MakeRotator (.roll _returnvalue) (.pitch _returnvalue) (.yaw (Math|Rotator|FindLookatRotation (Transformation|GetActorLocation) (Transformation|GetActorLocation (Variables|Default|GetClosest%20Player))))) _rotation true)))))))))

(event OnComponentBeginOverlap(Weapon01)
  (params (OverlappedComponent :type Primitive%20Component%20Object%20Reference) (OtherActor :type Actor%20Object%20Reference) (OtherComp :type Primitive%20Component%20Object%20Reference) (OtherBodyIndex :type Integer) (bFromSweep :type Boolean) (SweepResult :type Hit%20Result%20Structure%20%28by%20ref%29))
  (bind _asbp_lisa (Utilities|Casting|CastToBP_Lisa OtherActor))
  (if (not (Utilities|Array|ContainsItem (Variables|Default|GetAlreadyDamagedPlayers) _asbp_lisa))
    (Default|PlayerTakeDamage _asbp_lisa 1e+01 self)
    (Utilities|Array|Add (Variables|Default|GetAlreadyDamagedPlayers) _asbp_lisa)))

(event OnComponentBeginOverlap(Weapon02)
  (params (OverlappedComponent :type Primitive%20Component%20Object%20Reference) (OtherActor :type Actor%20Object%20Reference) (OtherComp :type Primitive%20Component%20Object%20Reference) (OtherBodyIndex :type Integer) (bFromSweep :type Boolean) (SweepResult :type Hit%20Result%20Structure%20%28by%20ref%29))
  (bind _asbp_lisa (Utilities|Casting|CastToBP_Lisa OtherActor))
  (if (not (Utilities|Array|ContainsItem (Variables|Default|GetAlreadyDamagedPlayers) _asbp_lisa))
    (Default|PlayerTakeDamage _asbp_lisa 1e+01 self)
    (Utilities|Array|Add (Variables|Default|GetAlreadyDamagedPlayers) _asbp_lisa)))

(event Custom|Event%20initiate%20combat
  ;[1 1 1] Comment
  (Variables|Default|SetHas%20Target true)
  (Class|KismetSystemLibrary|PauseTimer 0 "Look For Player")
  (if (.TargetClosestPlayer (Utilities|Struct|BreakS_AI_BehaviourDetails (.BehaviourDetails (Utilities|Struct|BreakS_AI_EnemyDetails (Variables|Default|GetEnemy%20Details)))))
    (AI|AIMoveTo self "0, 0, 0" (Variables|Default|GetClosest%20Player) 5.0 false
      (:OnSuccess
        (CallFunction|MCPlayMontage (Utilities|Array|Get(acopy) (Variables|Default|GetAttackMontage) (Variables|Default|GetAttack%20count)) "None" :!label _label)
        (Utilities|FlowControl|Delay (Variables|Default|GetAnimation%20Delay))
        (if (>= (Variables|Default|GetAttack%20count) (- (Utilities|Array|Length (Variables|Default|GetAttackMontage)) 1))
          (Variables|Default|SetAttack%20count 0)
          (else
            (Math|Integer|IncrementInt (Variables|Default|GetAttack%20count)
              (:%20%20
                _))))
        (Utilities|FlowControl|Delay 1.0)
        (CallFunction|EventRestartCombat))
      (:OnFail
        (CallFunction|EventRestartCombat :!label _label_2)))
    (else
      (AI|AIMoveTo self "0, 0, 0" (Variables|Default|GetFurthest%20Player) 1e+02 false
        (:OnSuccess
          (goto _label))
        (:OnFail
          (goto _label_2))))))

(event Custom|Event%20Restart%20Combat
  ;[1 1 1] Comment
  (if (.TargetClosestPlayer (Utilities|Struct|BreakS_AI_BehaviourDetails (.BehaviourDetails (Utilities|Struct|BreakS_AI_EnemyDetails (Variables|Default|GetEnemy%20Details)))))
    (AI|AIMoveTo self "0, 0, 0" (Variables|Default|GetClosest%20Player) 5.0 false
      (:OnSuccess
        (CallFunction|MCPlayMontage (Utilities|Array|Get(acopy) (Variables|Default|GetAttackMontage) (Variables|Default|GetAttack%20count)) "None" :!label _label)
        (Utilities|FlowControl|Delay (Variables|Default|GetAnimation%20Delay))
        (if (>= (Variables|Default|GetAttack%20count) (- (Utilities|Array|Length (Variables|Default|GetAttackMontage)) 1))
          (Variables|Default|SetAttack%20count 0)
          (else
            (Math|Integer|IncrementInt (Variables|Default|GetAttack%20count)
              (:%20%20
                _))))
        (Utilities|FlowControl|Delay 1.0)
        (CallFunction|EventRestartCombat))
      (:OnFail
        (CallFunction|EventRestartCombat :!label _label_2)))
    (else
      (AI|AIMoveTo self "0, 0, 0" (Variables|Default|GetFurthest%20Player) 1e+02 false
        (:OnSuccess
          (goto _label))
        (:OnFail
          (goto _label_2))))))

(event Custom|Attach%20Weapon
  (bind _enemy_details (Variables|Default|GetEnemy%20Details))
  (bind _attackdetails (Utilities|Struct|BreakS_AI_EnemyDetails _enemy_details))
  (bind (_weaponmesh01 _weaponmesh02 _01socketname _02socketname) (Utilities|Struct|BreakS_AI_AttackDetails _attackdetails))
  ;[1 1 1] Attach weapon
  (Components|StaticMesh|SetStaticMesh (Variables|Default|GetWeapon01) _weaponmesh01)
  (Components|StaticMesh|SetStaticMesh (Variables|Default|GetWeapon02) _weaponmesh02)
  (Transformation|AttachComponentToComponent (Variables|Default|GetWeapon01) (Variables|Character|GetMesh) _01socketname "SnapToTarget" "SnapToTarget" "SnapToTarget" true)
  (Transformation|AttachComponentToComponent (Variables|Default|GetWeapon02) (Variables|Character|GetMesh) _02socketname "SnapToTarget" "SnapToTarget" "SnapToTarget" true))

(fn ConstructionScript)

(fn AiTakeDamage
  (params (AttackingPlayer :type BP%20Lisa%20Object%20Reference) (Damage :type Float%20%28double-precision%29))
  (Development|PrintString "Damage Applied" true true "(R=1.000000,G=0.015359,B=0.000000,A=1.000000)" 0.5)
  (CallFunction|EventShowHealthBar)
  (Variables|Default|SetCurrentHealth (- (Variables|Default|GetCurrentHealth) Damage))
  (CallFunction|ServerPlayMontage (Utilities|Array|Get(acopy) (Variables|Default|GetDamage%20montage) (Variables|/Game/game_char/BP_Lisa.BP_Lisa_C|GetAssasin%20attack%20count AttackingPlayer)) "None"))

(fn SetupAIMovement
  (bind _enemy_details (Variables|Default|GetEnemy%20Details))
  (bind _movementdetails (Utilities|Struct|BreakS_AI_EnemyDetails _enemy_details))
  (bind (_animationblueprint _maxwalkspeed _maxrunspeed) (Utilities|Struct|BreakS_AI_MovementDetails _movementdetails))
  (Class|SkeletalMeshComponent|SetAnimClass (Variables|Character|GetMesh) _animationblueprint)
  (Variables|/Script/Engine.CharacterMovementComponent|SetMaxWalkSpeed (Variables|Character|GetCharacterMovement) _maxrunspeed))

(fn SetupAIStats
  (bind _output_get (Variables|Default|SetMaxHealth (Utilities|Struct|BreakS_AI_StatDetails (.statdetails (Utilities|Struct|BreakS_AI_EnemyDetails (Variables|Default|GetEnemy%20Details))))))
  (Variables|Default|SetCurrentHealth _output_get))

(fn SetupAIBehaviour
  (if (.Roaming? (Utilities|Struct|BreakS_AI_BehaviourDetails (.BehaviourDetails (Utilities|Struct|BreakS_AI_EnemyDetails (Variables|Default|GetEnemy%20Details)))))
    (CallFunction|EventStartRoaming)))

(fn FindClosestPlayer
  (Variables|Default|SetClosest%20Player%20Distance 5e+04)
  (Variables|Default|SetFurthest%20Player%20Distance 1e+02)
  (bind _outactors (Actor|GetAllActorsOfClass "/Game/game_char/BP_Lisa.BP_Lisa_C"))
  (for _array_element _outactors
    (if (< (Transformation|GetDistanceTo _array_element self) (Variables|Default|GetClosest%20Player%20Distance))
      (Variables|Default|SetClosest%20Player%20Distance (Transformation|GetDistanceTo _array_element self))
      (Variables|Default|SetClosest%20Player _array_element)
      (elif (> (Transformation|GetDistanceTo _array_element self) (Variables|Default|GetFurthest%20Player%20Distance))
        (Variables|Default|SetFurthest%20Player%20Distance (Transformation|GetDistanceTo _array_element self))
        (Variables|Default|SetFurthest%20Player _array_element)))))

(fn LookforPlayer
  (CallFunction|FindClosestPlayer)
  (if (< (Transformation|GetDistanceTo self (Variables|Default|GetClosest%20Player)) (.SeePlayerDistance (Utilities|Struct|BreakS_AI_BehaviourDetails (.BehaviourDetails (Utilities|Struct|BreakS_AI_EnemyDetails (Variables|Default|GetEnemy%20Details))))))
    (Development|PrintString "Ai Can See")
    (CallFunction|EventInitiateCombat)))